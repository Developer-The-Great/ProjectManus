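; ProjectManusPawnBP is a pawn Blueprint that tests receiving OSC messages through Unreal's OSC plugin.
; BeginPlay starts a listening server on port 12000 and binds any incoming message to a handler that only prints a fixed default string.
; An unconnected second setup would listen on port 9000 for "/wek/outputs" (apparently Wekinator) and print the float at index 1, but it never runs.
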(event Custom|OnMsgReceived
  (params (Message :type OSC%20Message%20Structure%20%28by%20ref%29) (IPAddress :type String) (Port :type Integer))
  ;[1 1 1] Binding to Any Message
  (Development|PrintString "Hello"))

(event Custom|OnMsgReceived_AddressPattern
  (params (AddressPattern :type OSC%20Address%20Structure%20%28by%20ref%29) (Message :type OSC%20Message%20Structure%20%28by%20ref%29) (IPAddress :type String) (Port :type Integer))
  ;[1 1 1] Binding to Address Pattern "/foo?1/slider*"
  (bind _value (Class|OSCManager|GetFloat Message 1))
  (Development|PrintString (Utilities|String|ToString(Float) _value)))

(event EventBeginPlay
  ;[1 1 1] Binding to Any Message
  (bind _returnvalue (Class|OSCManager|CreateOSCServer "" 12000 false true "" 0))
  ;[1 1 1] Binding to Address Pattern "/foo?1/slider*"
  (EventDispatchers|AssignOnOscMessageReceived _returnvalue (delegate Custom|OnMsgReceived)))

(fn ConstructionScript)