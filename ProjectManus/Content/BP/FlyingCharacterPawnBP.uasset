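; Flying character pawn Blueprint that receives four-float pose results over OSC and passes them to OnReceivePoseResults, which is not defined in this graph.
; BindOSC creates a listening OSC server on port 12000 and binds its message event, which unpacks the floats.
; BeginPlay runs this setup, and a Tick timer reruns it about every two seconds, creating a new server each time without storing it.
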(event Custom|OnMsgReceived
  (params (Message :type OSC%20Message%20Structure%20%28by%20ref%29) (IPAddress :type String) (Port :type Integer))
  ;[1 1 1] Binding to Any Message
  (bind _value (Class|OSCManager|GetFloat Message))
  (bind _value_2 (Class|OSCManager|GetFloat Message 1))
  (bind _value_3 (Class|OSCManager|GetFloat Message 2))
  (bind _value_4 (Class|OSCManager|GetFloat Message 3))
  (Class|FlyingCharacterPawn|OnReceivePoseResults (Utilities|Array|MakeArray _value _value_2 _value_3 _value_4)))

(event Custom|OnReInitServerEvent
  (CallFunction|BindOSC))

(event EventBeginPlay
  (CallFunction|OnReInitServerEvent))

(event EventTick
  (params (DeltaSeconds :type Float%20%28single-precision%29))
  (bind _output_get (Variables|Default|Settime (+ DeltaSeconds (Variables|Default|Gettime))))
  (Math|Float|CompareFloat _output_get 2.0
    (:>
      (CallFunction|OnReInitServerEvent)
      (Variables|Default|Settime (+ (Variables|Default|Gettime) (* (Variables|Default|Gettime) -1.0))))))

(fn ConstructionScript)

(fn BindOSC
  (bind _returnvalue (Class|OSCManager|CreateOSCServer "" 12000 false true "" 0))
  (EventDispatchers|BindEventtoOnOscMessageReceived _returnvalue (EventDispatchers|CreateEvent :!event Custom|OnMsgReceived))
  (Development|PrintString "OSCServerInitialized" true false))